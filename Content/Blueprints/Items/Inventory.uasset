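; Inventory Blueprint that holds a list of items and persists it through an InventorySave save game slot.
; BeginPlay restores Items from the slot if a save exists, then calls AddItem with no item specified.
; AddItem appends uniquely and prints the item's data name.
; SaveInventory writes Items to a new save object in that slot, but nothing in this Blueprint calls it.
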(event `self.ReceiveBeginPlay`
  (`self.LoadInventory`)
  (`self.AddItem` null))

(event `AddItem`
  (params (ItemToAdd :type "/Game/Blueprints/Items/Item Object Reference"))
  (bind _itemdata_name (break `/Game/Blueprints/Items/ItemData` (`/Game/Blueprints/Items/Item.ItemData` ItemToAdd)))
  (`KismetArrayLibrary.Array_AddUnique` (`self.Items`) ItemToAdd)
  (`KismetSystemLibrary.PrintString` _itemdata_name))

(fn `LoadInventory`
  (bind _returnvalue (`GameplayStatics.DoesSaveGameExist` (`self.InventroySaveSlot`)))
  (if _returnvalue
    (bind _returnvalue_2 (`GameplayStatics.LoadGameFromSlot` (`self.InventroySaveSlot`)))
    (bind _asinventory_save (cast `/Game/Blueprints/Items/InventorySave` _returnvalue_2))
    (set `self.Items` (`/Game/Blueprints/Items/InventorySave.SavedItems` _asinventory_save))))

(fn `SaveInventory`
  (locals (InventroySaveInfo :type "/Game/Blueprints/Items/InventorySave Object Reference"))
  (bind _returnvalue (`GameplayStatics.CreateSaveGameObject` "/Game/Blueprints/Items/InventorySave.InventorySave_C"))
  (bind _output_get (set `local.InventroySaveInfo` _returnvalue))
  (set `/Game/Blueprints/Items/InventorySave.SavedItems` (`self.Items`) _output_get)
  (`GameplayStatics.SaveGameToSlot` (`local.InventroySaveInfo`) (`self.InventroySaveSlot`)))

(fn `UserConstructionScript`)